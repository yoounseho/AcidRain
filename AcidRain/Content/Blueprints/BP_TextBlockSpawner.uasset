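; Spawner actor for an acid-rain text game that creates a falling-word block (BP_NewAcidRainBlock) on a looping timer started at BeginPlay.
; Each tick of the timer picks a random TextTable row and deprojects the game instance's screen-space spawn zone into world space, randomizing Y toward the viewport's edge.
; The block receives the row's KR text and is registered with BP_AcidRainGameInstance.
; CurrentLanguage is stored, but its language switch is disconnected.
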(event `SpawnTextBlock`
  (bind _returnvalue (`GameplayStatics.GetPlayerController` 0))
  (bind _returnvalue_x (`KismetMathLibrary.BreakVector2D` (`WidgetLayoutLibrary.GetViewportSize`)))
  (bind _texttable (`self.TextTable`))
  (bind _returnvalue_x_2 (`KismetMathLibrary.BreakVector` (`SceneComponent.K2_GetComponentLocation` (`self.DefaultSceneRoot`))))
  (bind _outrownames (`DataTableFunctionLibrary.GetDataTableRowNames` _texttable))
  (bind _returnvalue_2 (`|GetDataTableRow` _texttable (`|GetArrayItem` _outrownames (`KismetMathLibrary.RandomIntegerInRange` 0 (- (`KismetArrayLibrary.Array_Length` _outrownames) 1))))
    (:`then`
      (bind _asbp_acid_rain_game_instance (cast `/Game/Blueprints/BP_AcidRainGameInstance` (`GameplayStatics.GetGameInstance`)))
      (bind (_pos _returnval) (`/Game/Blueprints/BP_AcidRainGameInstance.GetSpawnZonePosition` _asbp_acid_rain_game_instance))
      (if _returnval
        (bind (_worldposition _worlddirection) (`GameplayStatics.DeprojectScreenToWorld` _returnvalue (`KismetMathLibrary.MakeVector2D` (`KismetMathLibrary.BreakVector2D` _pos) (`.Y` (`KismetMathLibrary.BreakVector2D` _pos)))))
        (bind (_returnvalue_x_3 _returnvalue_y) (`KismetMathLibrary.BreakVector` (+ _worldposition (* _worlddirection _returnvalue_x_2))))
        (bind (_worldposition_2 _worlddirection_2) (`GameplayStatics.DeprojectScreenToWorld` _returnvalue (`KismetMathLibrary.MakeVector2D` _returnvalue_x (`.Y` (`KismetMathLibrary.BreakVector2D` _pos)))))
        (bind (_returnvalue_x_4 _returnvalue_y_2 _returnvalue_z) (`KismetMathLibrary.BreakVector` (+ _worldposition_2 (* _worlddirection_2 _returnvalue_x_2))))
        (bind _returnvalue_3 (`|SpawnActorFromClass` "/Game/Blueprints/BP_NewAcidRainBlock.BP_NewAcidRainBlock_C" (`KismetMathLibrary.MakeTransform` (`KismetMathLibrary.MakeVector` _returnvalue_x_3 (`KismetMathLibrary.RandomFloatInRange` _returnvalue_y _returnvalue_y_2) _returnvalue_z) (.rotation (`self.GetTransform`))) "AlwaysSpawn" "OverrideRootScale" self null))
        (`/Game/Blueprints/BP_NewAcidRainBlock.Initialize` _returnvalue_3 (`.KR_5_54B28648448C90D377D24E963D380876` (break `/Game/Blueprints/FLocalizeTextStruct` _returnvalue_2)))
        (bind _asbp_acid_rain_game_instance_2 (cast `/Game/Blueprints/BP_AcidRainGameInstance` (`GameplayStatics.GetGameInstance`)))
        (`/Game/Blueprints/BP_AcidRainGameInstance.AssignTextBlock` _asbp_acid_rain_game_instance_2 _returnvalue_3)))))

(event `self.ReceiveBeginPlay`
  (set `self.CurrentLanguage` (`KismetInternationalizationLibrary.GetCurrentLanguage`))
  (bind _returnvalue (`KismetSystemLibrary.K2_SetTimerDelegate` (delegate `SpawnTextBlock`) 2.0 true))
  (set `self.SpawnHandle` _returnvalue))

(event `self.ReceiveTick`
  (params (DeltaSeconds :type "Float (single-precision)")))

(fn `UserConstructionScript`)
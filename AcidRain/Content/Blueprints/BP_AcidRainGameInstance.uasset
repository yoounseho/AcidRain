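; Game instance for an acid rain word game that tracks text blocks and the spawn and dead zone positions.
; Blocks register through an event; HitBlock destroys the first block matching the given text but removes array index 0, not the matched index.
; Zone setters raise initialized flags, which the getters return as validity alongside the position.
; Reset clears the flags, positions and block list.
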(event `AssignTextBlock`
  (params (Block :type "/Game/Blueprints/BP_NewAcidRainBlock Object Reference"))
  (`KismetArrayLibrary.Array_Add` (`self.AssignedTexts`) Block))

(fn `GetDeadZonePosition`
  (returns (Pos :type "Vector2D Structure") (ReturnVal :type Boolean))
  (if (`self.bInitializedDeadZone`)
    (return (`self.DeadZonePosition`) true)
    (else
      (return (0.0 0.0) false))))

(fn `GetSpawnZonePosition`
  (returns (Pos :type "Vector2D Structure") (ReturnVal :type Boolean))
  (if (`self.bInitializedSpawnZone`)
    (return (`self.SpawnZonePosition`) true)
    (else
      (return (0.0 0.0) false))))

(fn `HitBlock`
  (params (Text :type Text))
  (bind _assignedtexts (`self.AssignedTexts`))
  (bind (_returnvalue _index) (`self.SearchText` Text))
  (if _returnvalue
    (`Actor.K2_DestroyActor` (`|GetArrayItem` _assignedtexts _index))
    (`KismetArrayLibrary.Array_Remove` _assignedtexts)))

(fn `InitializeDeadZonePosition`
  (params (Pos :type "Vector2D Structure"))
  (set `self.DeadZonePosition` Pos)
  (set `self.bInitializedDeadZone` true))

(fn `InitializeSpawnZonePosition`
  (params (Pos :type "Vector2D Structure"))
  (set `self.SpawnZonePosition` Pos)
  (set `self.bInitializedSpawnZone` true))

(fn `Reset`
  (set `self.bInitializedSpawnZone` false)
  (set `self.bInitializedDeadZone` false)
  (set `self.SpawnZonePosition` (0.0 0.0))
  (set `self.DeadZonePosition` (0.0 0.0))
  (`KismetArrayLibrary.Array_Clear` (`self.AssignedTexts`)))

(fn `SearchText`
  (params (Text :type Text))
  (returns (ReturnValue :type Boolean) (Index :type Integer))
  (for (_array_element _array_index) (`self.AssignedTexts`)
    (if (`KismetTextLibrary.EqualEqual_TextText` (`/Game/Blueprints/BP_NewAcidRainBlock.Text` _array_element) Text)
      (return true _array_index)))
  (return false -1))
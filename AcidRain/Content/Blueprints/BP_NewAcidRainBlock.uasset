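; BP_NewAcidRainBlock is a falling text block actor for an acid rain game, showing its text on a widget component.
; Initialize writes the text into the UMG_TextBlock widget, stores it and turns on physics simulation so the widget moves.
; Each tick it projects the widget to screen space and destroys itself once it drops below the dead zone position held by BP_AcidRainGameInstance.
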(event `Initialize`
  (params (Text :type Text))
  (bind _widget (`self.Widget`))
  (bind _asumg_text_block (cast `/Game/Blueprints/UMG_TextBlock` (`WidgetComponent.GetUserWidgetObject` _widget)))
  (`/Game/Blueprints/UMG_TextBlock.SetText` _asumg_text_block Text)
  (`PrimitiveComponent.SetSimulatePhysics` _widget true)
  (set `self.Text` Text))

(event `self.ReceiveBeginPlay`)

(event `self.ReceiveTick`
  (params (DeltaSeconds :type "Float (single-precision)"))
  (bind _output_get (set `self.ViewPortPosition` (`WidgetLayoutLibrary.ProjectWorldLocationToWidgetPosition` (`GameplayStatics.GetPlayerController` 0) (`SceneComponent.K2_GetComponentLocation` (`self.Widget`)))))
  (bind _asbp_acid_rain_game_instance (cast `/Game/Blueprints/BP_AcidRainGameInstance` (`GameplayStatics.GetGameInstance`)))
  (bind (_pos _returnval) (`/Game/Blueprints/BP_AcidRainGameInstance.GetDeadZonePosition` _asbp_acid_rain_game_instance))
  (if _returnval
    (if (> (`.Y` (`KismetMathLibrary.BreakVector2D` _output_get)) (`.Y` (`KismetMathLibrary.BreakVector2D` _pos)))
      (`self.K2_DestroyActor`))))

(fn `UserConstructionScript`)